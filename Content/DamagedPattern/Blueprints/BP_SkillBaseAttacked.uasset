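; BP_SkillBaseAttacked is a hit-reaction actor that knocks back an iron golem struck by an arrow.
; Play takes the arrow's normalized fixed vector as direction, then fires the OnActorShaked dispatcher.
; Its handler sets the golem's IsDamaged flag to block overlapping reactions, then uses a Timeline for swept horizontal movement and curve-driven height.
; When the Timeline finishes, it clears the flag and destroys itself.
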(event Custom|OnActorShaked_Event
  (bind _attackedactordirection (Variables|Default|GetAttackedActorDirection))
  (bind _asbp_iron_golem (Utilities|Casting|CastTobp_ironGolem (Variables|Default|GetDamagedActor)))
  (if (Variables|/Game/monster/bp_ironGolem.bp_ironGolem_C|GetisDamaged _asbp_iron_golem)
    (Development|PrintString "Is Shaking")
    (else
      (Variables|/Game/monster/bp_ironGolem.bp_ironGolem_C|SetisDamaged _asbp_iron_golem true)
      (Variables|Default|SetDirection2D (Math|Vector2D|MakeVector2D (.x _attackedactordirection) (.y _attackedactordirection)))
      (bind _output_get (Variables|Default|SetStartZ (.z (Transformation|GetActorLocation (Variables|Default|GetDamagedActor)))))
      (Variables|Default|SetTargetZ (+ _output_get 1e+02))
      (bind _shaking (Timeline|Timeline Play)
        (:Update
          (Transformation|SetActorLocation (Variables|Default|GetDamagedActor) (Math|Vector|MakeVector (.x (+ (Transformation|GetActorLocation (Variables|Default|GetDamagedActor)) (Math|Vector|MakeVector (.x (* (* (Variables|Default|GetDirection2D) (Variables|Default|GetKnockBackSpeed)) (Utilities|Time|GetWorldDeltaSeconds))) (.y (* (* (Variables|Default|GetDirection2D) (Variables|Default|GetKnockBackSpeed)) (Utilities|Time|GetWorldDeltaSeconds))) 0.0))) (.y (+ (Transformation|GetActorLocation (Variables|Default|GetDamagedActor)) (Math|Vector|MakeVector (.x (* (* (Variables|Default|GetDirection2D) (Variables|Default|GetKnockBackSpeed)) (Utilities|Time|GetWorldDeltaSeconds))) (.y (* (* (Variables|Default|GetDirection2D) (Variables|Default|GetKnockBackSpeed)) (Utilities|Time|GetWorldDeltaSeconds))) 0.0))) (Math|Float|Lerp (Variables|Default|GetStartZ) (Variables|Default|GetTargetZ) _shaking)) true false))
        (:Finished
          (Variables|/Game/monster/bp_ironGolem.bp_ironGolem_C|SetisDamaged _asbp_iron_golem false)
          (Actor|DestroyActor))))))

(event EventBeginPlay
  (EventDispatchers|BindEventtoOnActorShaked (delegate Custom|OnActorShaked_Event)))

(event Collision|EventActorBeginOverlap
  (params (OtherActor :type Actor%20Object%20Reference))
  (|CallParentFunction OtherActor) ; This node is disabled and will not be called.\nDrag off pins to build functionality.
)

(event EventTick
  (params (DeltaSeconds :type Float%20%28single-precision%29))
  (|CallParentFunction DeltaSeconds) ; This node is disabled and will not be called.\nDrag off pins to build functionality.
)

(fn ConstructionScript
  (|CallParentFunction))

(fn Play
  (params (DamagedActor :type Actor%20Object%20Reference) (AttackingActor :type Actor%20Object%20Reference))
  (Variables|Default|SetDamagedActor DamagedActor)
  (Variables|Default|SetAttackingActor AttackingActor)
  (bind _asbp_arrow (Utilities|Casting|CastToBP_Arrow AttackingActor))
  (Variables|Default|SetAttackedActorDirection (Math|Vector|Normalize (Variables|/Game/Player/BluePrints/Skill/BP_Arrow.BP_Arrow_C|GetFixed%20Vector%20with%20Speed _asbp_arrow)))
  (Default|CallOnActorShaked))