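; BP_SkillFreeze is a skill in the damaged-pattern set that freezes a hit BP_Steve in place for a few seconds.
; Play passes the damaged actor to freezeEvent, which skips flying targets, spawns a Bp_ice at the target and disables its movement mode.
; After a delay it restores Walking and destroys the ice, printing debug messages at freeze and melt.
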(event Custom|freezeEvent
  (params (damagedActor :type Actor%20Object%20Reference))
  (bind _asbp_steve (Utilities|Casting|CastToBP_Steve damagedActor))
  (if (not (Class|NavMovementInterface|IsFlying (Variables|/Script/Engine.Character|GetCharacterMovement _asbp_steve)))
    (Development|PrintString "freeze!")
    (bind _returnvalue (Game|SpawnActorfromClass "/Game/monster/skill/object/bp_ice.bp_ice_C" (Transformation|GetActorTransform _asbp_steve) "Undefined" "MultiplyWithRoot" 0 0))
    (Pawn|Components|CharacterMovement|SetMovementMode (Variables|/Script/Engine.Character|GetCharacterMovement _asbp_steve) "MOVE_None" 0)
    (Utilities|FlowControl|Delay 4.0)
    (Pawn|Components|CharacterMovement|SetMovementMode (Variables|/Script/Engine.Character|GetCharacterMovement _asbp_steve) "MOVE_Walking" 0)
    (Actor|DestroyActor _returnvalue)
    (Development|PrintString "melt")))

(event EventBeginPlay)

(event Collision|EventActorBeginOverlap
  (params (OtherActor :type Actor%20Object%20Reference)))

(event EventTick
  (params (DeltaSeconds :type Float%20%28single-precision%29)))

(fn ConstructionScript
  (|CallParentFunction))

(fn Play
  (params (DamagedActor :type Actor%20Object%20Reference) (AttackingActor :type Actor%20Object%20Reference))
  (CallFunction|FreezeEvent DamagedActor))