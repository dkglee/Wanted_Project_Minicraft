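; BP_SkillFreeze is an Iron Golem damage-pattern skill that freezes a damaged BP_Steve in place for a few seconds.
; Play triggers the freeze, which is skipped if a BP_SkillThrowPattern actor exists.
; Otherwise it spawns Bp_ice, attaches it to Steve's mesh root socket and disables Moveable.
; After a delay it restores movement, destroys every Bp_ice in the level and then itself.
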(event Custom|freezeEvent
  (params (damagedActor :type Actor%20Object%20Reference))
  (bind _asbp_steve (Utilities|Casting|CastToBP_Steve damagedActor))
  (Variables|Default|SetAs%20BP%20Steve _asbp_steve)
  (bind _returnvalue (Actor|GetActorOfClass "/Game/DamagedPattern/Blueprints/ironGolem/BP_SkillThrowPattern.BP_SkillThrowPattern_C"))
  (Utilities|IsValid _returnvalue
    (:Is%20Valid
      (Development|PrintString "thrown"))
    (:Is%20Not%20Valid
      (Development|PrintString "freeze!")
      (bind _returnvalue_2 (Game|SpawnActorfromClass "/Game/monster/skill/object/bp_ice.bp_ice_C" (Transformation|GetActorTransform (Variables|Default|GetAs%20BP%20Steve)) "Undefined" "MultiplyWithRoot" 0 0))
      (Utilities|IsValid _returnvalue_2
        (:Is%20Valid
          (Transformation|AttachComponentToComponent _returnvalue_2 (Variables|/Script/Engine.Character|GetMesh (Variables|Default|GetAs%20BP%20Steve)) "ROOTSocket" "KeepWorld" "KeepWorld" "KeepWorld" true)
          (Variables|/Game/Player/BluePrints/BP_Steve.BP_Steve_C|SetbMoveable (Variables|Default|GetAs%20BP%20Steve) false)
          (Utilities|FlowControl|Delay 4.0)
          (Variables|/Game/Player/BluePrints/BP_Steve.BP_Steve_C|SetbMoveable (Variables|Default|GetAs%20BP%20Steve) true)
          (bind _outactors (Actor|GetAllActorsOfClass "/Game/monster/skill/object/bp_ice.bp_ice_C"))
          (for _array_element _outactors
            (Utilities|IsValid _array_element
              (:Is%20Valid
                (Actor|DestroyActor _array_element))))
          (Development|PrintString "melt")
          (Actor|DestroyActor))))))

(event EventBeginPlay)

(event Collision|EventActorBeginOverlap
  (params (OtherActor :type Actor%20Object%20Reference)))

(event EventTick
  (params (DeltaSeconds :type Float%20%28single-precision%29)))

(fn ConstructionScript
  (|CallParentFunction))

(fn Play
  (params (DamagedActor :type Actor%20Object%20Reference) (AttackingActor :type Actor%20Object%20Reference))
  (CallFunction|FreezeEvent DamagedActor))