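; Damage pattern actor for the Iron Golem's base attack, which flags a hit BP_Steve as damaged.
; Play forwards the damaged actor to baseAttackEvent and leaves the attacking actor unused.
; If Steve is not already damaged, the event pulses IsDamaged for one tick, then destroys this actor.
; A failed cast or already-damaged Steve leaves the actor alive.
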(event Custom|baseAttackEvent
  (params (damagedActor :type Actor%20Object%20Reference))
  (bind _asbp_steve (Utilities|Casting|CastToBP_Steve damagedActor))
  (Variables|Default|SetAs%20BP%20Steve _asbp_steve)
  (if (not (Variables|/Game/Player/BluePrints/BP_Steve.BP_Steve_C|GetbIsDamaged (Variables|Default|GetAs%20BP%20Steve)))
    (Variables|/Game/Player/BluePrints/BP_Steve.BP_Steve_C|SetbIsDamaged (Variables|Default|GetAs%20BP%20Steve) true)
    (Utilities|FlowControl|DelayUntilNextTick)
    (Variables|/Game/Player/BluePrints/BP_Steve.BP_Steve_C|SetbIsDamaged (Variables|Default|GetAs%20BP%20Steve) false)
    (Actor|DestroyActor)))

(event EventBeginPlay)

(event Collision|EventActorBeginOverlap
  (params (OtherActor :type Actor%20Object%20Reference)))

(event EventTick
  (params (DeltaSeconds :type Float%20%28single-precision%29)))

(fn ConstructionScript
  (|CallParentFunction))

(fn Play
  (params (DamagedActor :type Actor%20Object%20Reference) (AttackingActor :type Actor%20Object%20Reference))
  (CallFunction|BaseAttackEvent DamagedActor))