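; Damage pattern actor for the Iron Golem's throw skill, which flings a hit BP_Steve into the air.
; Play triggers throwEvent, which skips targets already flagged IsDamaged and finds the golem via GetActorOfClass rather than the passed attacker.
; A timeline lerps Steve's location forward along the golem's facing and upward, without sweep.
; On completion it clears the flag and destroys itself.
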(event Custom|throwEvent
  (params (damagedActor :type Actor%20Object%20Reference) (attackActor :type Actor%20Object%20Reference))
  (bind _returnvalue (Actor|GetActorOfClass "/Game/monster/bp_ironGolem.bp_ironGolem_C"))
  (Variables|Default|SetAs%20BP%20IronGolem _returnvalue)
  (bind _asbp_steve (Utilities|Casting|CastToBP_Steve damagedActor))
  (bind _output_get (Variables|Default|SetAs%20BP%20Steve _asbp_steve))
  (if (not (Variables|/Game/Player/BluePrints/BP_Steve.BP_Steve_C|GetbIsDamaged _output_get))
    (Variables|/Game/Player/BluePrints/BP_Steve.BP_Steve_C|SetbIsDamaged _output_get true)
    (Variables|Default|Setstart (Transformation|GetActorLocation (Variables|Default|GetAs%20BP%20Steve)))
    (Variables|Default|Setend (Math|Vector|MakeVector (+ (.x (* (Transformation|GetActorForwardVector (Variables|Default|GetAs%20BP%20IronGolem)) 5e+02)) (.x (Variables|Default|Getstart))) (+ (.y (* (Transformation|GetActorForwardVector (Variables|Default|GetAs%20BP%20IronGolem)) 5e+02)) (.y (Variables|Default|Getstart))) (+ 1.5e+03 (.z (Variables|Default|Getstart)))))
    (bind _move (Timeline|Timeline Play)
      (:Update
        (Transformation|SetActorLocation (Variables|Default|GetAs%20BP%20Steve) (Math|Vector|Lerp(Vector) (Variables|Default|Getstart) (Variables|Default|Getend) _move) false false))
      (:Finished
        (Variables|/Game/Player/BluePrints/BP_Steve.BP_Steve_C|SetbIsDamaged (Variables|Default|GetAs%20BP%20Steve) false)
        (Actor|DestroyActor)))))

(event EventBeginPlay)

(event Collision|EventActorBeginOverlap
  (params (OtherActor :type Actor%20Object%20Reference)))

(event EventTick
  (params (DeltaSeconds :type Float%20%28single-precision%29)))

(fn ConstructionScript
  (|CallParentFunction))

(fn Play
  (params (DamagedActor :type Actor%20Object%20Reference) (AttackingActor :type Actor%20Object%20Reference))
  (CallFunction|ThrowEvent DamagedActor AttackingActor))