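; Hit-reaction actor that launches BP_Steve away from an attacking iron golem.
; Play forwards both actors to hitEvent, which skips an already-damaged Steve, otherwise sets IsDamaged and spawns blood Niagara effects.
; The Fly timeline lerps his location outward and upward using separate XY and Z curves.
; When the timeline finishes, it clears IsDamaged and destroys itself.
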(event Custom|hitEvent
  (params (damagedActor :type Actor%20Object%20Reference) (attackActor :type Actor%20Object%20Reference))
  (bind _asbp_iron_golem (Utilities|Casting|CastTobp_ironGolem attackActor))
  (Variables|Default|SetAs%20Bp%20Iron%20Golem _asbp_iron_golem)
  (bind _asbp_steve (Utilities|Casting|CastToBP_Steve damagedActor))
  (Variables|Default|SetAs%20BP%20Steve _asbp_steve)
  (if (not (Variables|/Game/Player/BluePrints/BP_Steve.BP_Steve_C|GetbIsDamaged (Variables|Default|GetAs%20BP%20Steve)))
    (Variables|/Game/Player/BluePrints/BP_Steve.BP_Steve_C|SetbIsDamaged (Variables|Default|GetAs%20BP%20Steve) true)
    (Niagara|SpawnSystematLocation "/Game/monster/effect/ns_blood.ns_blood" (Math|Vector|MakeVector (.x (Transformation|GetActorLocation (Variables|Default|GetAs%20BP%20Steve))) (.y (Transformation|GetActorLocation (Variables|Default|GetAs%20BP%20Steve))) (+ (.z (Transformation|GetActorLocation (Variables|Default|GetAs%20BP%20Steve))) 5e+01)))
    (Variables|Default|Setstart (Transformation|GetActorLocation (Variables|Default|GetAs%20BP%20Steve)))
    (Variables|Default|Setend (+ (Transformation|GetActorLocation (Variables|Default|GetAs%20BP%20Steve)) (Math|Vector|MakeVector (.x (* (Math|Vector|Normalize (Math|Vector|MakeVector (- (.x (Transformation|GetActorLocation (Variables|Default|GetAs%20BP%20Steve))) (.x (Transformation|GetActorLocation (Variables|Default|GetAs%20Bp%20Iron%20Golem)))) (- (.y (Transformation|GetActorLocation (Variables|Default|GetAs%20BP%20Steve))) (.y (Transformation|GetActorLocation (Variables|Default|GetAs%20Bp%20Iron%20Golem)))) 0.0)) 3e+02)) (.y (* (Math|Vector|Normalize (Math|Vector|MakeVector (- (.x (Transformation|GetActorLocation (Variables|Default|GetAs%20BP%20Steve))) (.x (Transformation|GetActorLocation (Variables|Default|GetAs%20Bp%20Iron%20Golem)))) (- (.y (Transformation|GetActorLocation (Variables|Default|GetAs%20BP%20Steve))) (.y (Transformation|GetActorLocation (Variables|Default|GetAs%20Bp%20Iron%20Golem)))) 0.0)) 3e+02)) 3e+02)))
    (bind (_direction _z _x__y) (Timeline|fly PlayFromStart)
      (:Update
        (Transformation|SetActorLocation (Variables|Default|GetAs%20BP%20Steve) (Math|Vector|MakeVector (Math|Float|Lerp (.x (Variables|Default|Getstart)) (.x (Variables|Default|Getend)) _x__y) (Math|Float|Lerp (.y (Variables|Default|Getstart)) (.y (Variables|Default|Getend)) _x__y) (Math|Float|Lerp (.z (Variables|Default|Getstart)) (.z (Variables|Default|Getend)) _z)) false false))
      (:Finished
        (Variables|/Game/Player/BluePrints/BP_Steve.BP_Steve_C|SetbIsDamaged (Variables|Default|GetAs%20BP%20Steve) false)
        (Actor|DestroyActor)))))

(event EventBeginPlay)

(event Collision|EventActorBeginOverlap
  (params (OtherActor :type Actor%20Object%20Reference)))

(event EventTick
  (params (DeltaSeconds :type Float%20%28single-precision%29)))

(fn ConstructionScript
  (|CallParentFunction))

(fn Play
  (params (DamagedActor :type Actor%20Object%20Reference) (AttackingActor :type Actor%20Object%20Reference))
  (CallFunction|HitEvent DamagedActor AttackingActor))