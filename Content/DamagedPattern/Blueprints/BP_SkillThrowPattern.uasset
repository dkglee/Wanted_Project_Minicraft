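; Damage-pattern Blueprint for a throw skill that launches the damaged actor, acting only on BP_Steve characters.
; Play forwards the actor to throwEvent, which switches its movement to Flying and applies a mass-independent impulse along the forward vector of ThrowArrowTemp.
; After a short delay, movement is set back to Walking.
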(event Custom|throwEvent
  (params (damagedActor :type Actor%20Object%20Reference))
  (bind _asbp_steve (Utilities|Casting|CastToBP_Steve damagedActor))
  (Pawn|Components|CharacterMovement|SetMovementMode (Variables|/Script/Engine.Character|GetCharacterMovement _asbp_steve) "MOVE_Flying" 0)
  (Physics|AddImpulse (Variables|/Script/Engine.Character|GetCharacterMovement _asbp_steve) (* (Math|Vector|GetForwardVector (Variables|Default|GetThrowArrowTemp)) 1.5e+03) true)
  (Utilities|FlowControl|Delay 1.0)
  (Pawn|Components|CharacterMovement|SetMovementMode (Variables|/Script/Engine.Character|GetCharacterMovement _asbp_steve) "MOVE_Walking" 0))

(event EventBeginPlay)

(event Collision|EventActorBeginOverlap
  (params (OtherActor :type Actor%20Object%20Reference)))

(event EventTick
  (params (DeltaSeconds :type Float%20%28single-precision%29)))

(fn ConstructionScript
  (|CallParentFunction))

(fn Play
  (params (DamagedActor :type Actor%20Object%20Reference))
  (CallFunction|ThrowEvent DamagedActor))