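; Map Blueprint that lays out a flat grid of instanced mesh tiles in a square spiral from the world origin at construction time.
; The construction script walks runs of Length-spaced steps, alternating between X and Y, with Count setting the number of runs.
; After each X run the step sign flips and FrontValue grows, widening the spiral.
; Instances use world space, and the event graph has no active logic.
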(event EventBeginPlay)

(event Collision|EventActorBeginOverlap
  (params (OtherActor :type Actor%20Object%20Reference)))

(event EventTick
  (params (DeltaSeconds :type Float%20%28single-precision%29)))

(fn ConstructionScript
  (Components|InstancedStaticMesh|AddInstance (Variables|Default|GetInstancedStaticMesh) (Math|Transform|MakeTransform "0, 0, 0") true)
  (for _index (range 0 (Variables|Default|Getcount))
    (Variables|Default|SetIndex _index)
    (for _index_2 (range 0 (Variables|Default|GetfrontValue))
      (if (== (Math|Integer|%(Integer) (Variables|Default|GetIndex) 2) 0)
        (Variables|Default|SetvectorX (+ (* (Variables|Default|Getsign) (Variables|Default|Getlength)) (Variables|Default|GetvectorX)))
        (else
          (Variables|Default|SetvectorY (+ (* (Variables|Default|Getsign) (Variables|Default|Getlength)) (Variables|Default|GetvectorY)))))
      (Components|InstancedStaticMesh|AddInstance (Variables|Default|GetInstancedStaticMesh) (Math|Transform|MakeTransform (Math|Vector|MakeVector (Math|Conversions|ToFloat(Integer) (Variables|Default|GetvectorX)) (Math|Conversions|ToFloat(Integer) (Variables|Default|GetvectorY)) 0.0)) true))
    (if (== (Math|Integer|%(Integer) (Variables|Default|GetIndex) 2) 0)
      (Math|Integer|IncrementInt (Variables|Default|GetfrontValue)
        (:%20%20
          (Variables|Default|Setsign (* (Variables|Default|Getsign) -1)))))))