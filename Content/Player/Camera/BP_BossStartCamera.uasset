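; Boss intro cinematic camera actor that takes over the player's view through StartCamera and flies along a spline.
; MoveCamera snaps the camera to the spline's end, holds briefly, then a timeline scaled by PlayerTime moves it backward to near the start, following spline location and rotation.
; When the move finishes, it starts the Bp_golemAppear actor; the logic handing view back to BP_Steve is unconnected.
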(event Custom|Move%20Camera
  (bind _spline (Variables|Default|GetSpline))
  (bind _spline_2 (Variables|Default|GetSpline))
  (bind _returnvalue (Spline|GetSplineLength _spline))
  (Components|Timeline|SetPlayRate (Variables|Default|GetCamera%20Move%20Time) (/ 1.0 (Variables|Default|GetPlayer%20Time)))
  (Transformation|SetRelativeTransform (Variables|Default|GetBossCinemaCamera) (Math|Transform|MakeTransform (Spline|GetLocationatDistanceAlongSpline _spline _returnvalue "Local") (Spline|GetRotationatDistanceAlongSpline _spline _returnvalue "Local") "1.000000,1.000000,1.000000") false false)
  (Utilities|FlowControl|Delay 2.0)
  (bind _newtrack_0 (Timeline|Camera%20Move%20Time PlayFromStart)
    (:Update
      (Transformation|SetRelativeTransform (Variables|Default|GetBossCinemaCamera) (Math|Transform|MakeTransform (Spline|GetLocationatDistanceAlongSpline _spline_2 (Math|Float|Lerp (Spline|GetSplineLength (Variables|Default|GetSpline)) 3.5e+02 _newtrack_0) "Local") (Spline|GetRotationatDistanceAlongSpline _spline_2 (Math|Float|Lerp (Spline|GetSplineLength (Variables|Default|GetSpline)) 3.5e+02 _newtrack_0) "Local") "1.000000,1.000000,1.000000") false false))
    (:Finished
      (bind _returnvalue_2 (Actor|GetActorOfClass "/Game/monster/bp_golemAppear.bp_golemAppear_C"))
      (Default|Start _returnvalue_2))))

(event EventBeginPlay)

(event Collision|EventActorBeginOverlap
  (params (OtherActor :type Actor%20Object%20Reference)))

(event EventTick
  (params (DeltaSeconds :type Float%20%28single-precision%29)))

(fn ConstructionScript)

(fn StartCamera
  (Game|Player|SetViewTargetwithBlend (Game|GetPlayerController 0) self 0.0 "VTBlend_Linear" 0.0 false)
  (CallFunction|MoveCamera))