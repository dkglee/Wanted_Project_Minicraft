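; Player sound component that throttles attack sounds per index so repeated calls do not replay them each time.
; BeginPlay fills a flag array; PlayAttackSound plays explosion and magic cues when the index's flag is clear, then sets it.
; Later calls only increment counters, clearing the flag after two calls, or four for indices above 24.
; Those higher indices count and clear at index modulo 25, not the original slot.
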(event EventBeginPlay
  (for _index (range 0 25)
    (Utilities|Array|Add (Variables|Default|GetBasicSkillArrowMap) false)))

(event EventTick
  (params (DeltaSeconds :type Float%20%28single-precision%29)))

(fn PlayAttackSound
  (params (index :type Integer))
  (bind _count (Variables|Default|GetCount))
  (bind _countstrong (Variables|Default|GetCountStrong))
  (LocalVariables|Setindex_local index)
  (if (Utilities|Array|Get(acopy) (Variables|Default|GetBasicSkillArrowMap) (LocalVariables|Getindex_local))
    (if (> (LocalVariables|Getindex_local) 24)
      (LocalVariables|Setindex_local (Math|Integer|%(Integer) (LocalVariables|Getindex_local) 25))
      (Utilities|Array|SetArrayElem _countstrong (LocalVariables|Getindex_local) (+ (Utilities|Array|Get(acopy) _countstrong (LocalVariables|Getindex_local)) 1))
      (if (>= (Utilities|Array|Get(acopy) _countstrong (LocalVariables|Getindex_local)) 4)
        (Utilities|Array|SetArrayElem (Variables|Default|GetBasicSkillArrowMap) (LocalVariables|Getindex_local) false)
        (Utilities|Array|SetArrayElem (Variables|Default|GetCountStrong) (LocalVariables|Getindex_local) 0))
      (else
        (Utilities|Array|SetArrayElem _count (LocalVariables|Getindex_local) (+ (Utilities|Array|Get(acopy) _count (LocalVariables|Getindex_local)) 1))
        (if (>= (Utilities|Array|Get(acopy) _count (LocalVariables|Getindex_local)) 2)
          (Utilities|Array|SetArrayElem (Variables|Default|GetBasicSkillArrowMap) (LocalVariables|Getindex_local) false)
          (Utilities|Array|SetArrayElem (Variables|Default|GetCount) (LocalVariables|Getindex_local) 0))))
    (else
      (Audio|PlaySound2D "/Game/Player/Sound/Explosion_Large_1-1_Cue.Explosion_Large_1-1_Cue" 0.3 1.0 0.0 0 0)
      (Audio|PlaySound2D "/Game/Player/Sound/Magical_Interface_5-1_Cue.Magical_Interface_5-1_Cue" 0.1 1.0 0.0 0 0)
      (Utilities|Array|SetArrayElem (Variables|Default|GetBasicSkillArrowMap) (LocalVariables|Getindex_local) true))))