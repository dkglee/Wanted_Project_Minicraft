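; C_Player is the third-person player character, handling Enhanced Input for movement, jumping, camera look and a toggled zoom.
; It adds the player mapping context on controller change and clamps camera pitch on BeginPlay.
; Zoom switches the spring arm's socket offset.
; Each Tick, it faces the controller direction when zooming or when velocity aligns with control yaw above a dot-product threshold, otherwise orienting to movement.
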(event Input|EnhancedActionEvents|EnhancedInputActionIA_Player_Zoom
  (params (ActionValue :type Boolean) (ElapsedSeconds :type Float%20%28double-precision%29) (TriggeredSeconds :type Float%20%28double-precision%29) (InputAction :type Input%20Action%20Object%20Reference :default "/Game/Player/Input/Actions/IA_Player_Zoom.IA_Player_Zoom"))
  (bind _springarm (Variables|Default|GetSpringArm))
  (:Started
    (Development|PrintString "Hello")
    (bind _output_get (Variables|Default|SetbZooming (not (Variables|Default|GetbZooming))))
    (if _output_get
      (Variables|/Script/Engine.SpringArmComponent|SetSocketOffset _springarm "-150.000000,50.000000,100.000000")
      (else
        (Variables|/Script/Engine.SpringArmComponent|SetSocketOffset _springarm (Variables|Default|GetDefualtCameraSocketOffset))))))

(event Input|EnhancedActionEvents|EnhancedInputActionIA_Player_Move
  (params (ActionValue :type Vector%202D%20Structure) (ElapsedSeconds :type Float%20%28double-precision%29) (TriggeredSeconds :type Float%20%28double-precision%29) (InputAction :type Input%20Action%20Object%20Reference :default "/Game/Player/Input/Actions/IA_Player_Move.IA_Player_Move"))
  (bind _returnvalue (Pawn|GetControlRotation :!class /Script/Engine.Pawn))
  ;[0.15 0.15 0.15 0.5] Logic For Player Move
  (Pawn|Input|AddMovementInput (Math|Vector|GetRightVector (Math|Rotator|MakeRotator (.roll _returnvalue) 0.0 (.yaw _returnvalue))) (.x ActionValue) false)
  (Pawn|Input|AddMovementInput (Math|Vector|GetForwardVector (Math|Rotator|MakeRotator 0.0 0.0 (.yaw (Pawn|GetControlRotation :!class /Script/Engine.Pawn)))) (.y ActionValue) false))

(event Input|EnhancedActionEvents|EnhancedInputActionIA_Player_Jump
  (params (ActionValue :type Boolean) (ElapsedSeconds :type Float%20%28double-precision%29) (TriggeredSeconds :type Float%20%28double-precision%29) (InputAction :type Input%20Action%20Object%20Reference :default "/Game/Player/Input/Actions/IA_Player_Jump.IA_Player_Jump"))
  ;[0.15 0.15 0.15 0.5] Logic for Player Jump
  (:Started
    (Character|Jump))
  (:Completed
    (Character|StopJumping)))

(event Input|EnhancedActionEvents|EnhancedInputActionIA_Player_Look
  (params (ActionValue :type Vector%202D%20Structure) (ElapsedSeconds :type Float%20%28double-precision%29) (TriggeredSeconds :type Float%20%28double-precision%29) (InputAction :type Input%20Action%20Object%20Reference :default "/Game/Player/Input/Actions/IA_Player_Look.IA_Player_Look"))
  ;[0.15 0.15 0.15 0.5] Logic for Camera Input
  ;;[0.15 0.15 0.15 0.5] Left/Right Look
  (Pawn|Input|AddControllerYawInput (.x ActionValue))
  ;;[0.15 0.15 0.15 0.5] Up/Down Look
  (Pawn|Input|AddControllerPitchInput (.y ActionValue)))

(event EventBeginPlay
  (bind _returnvalue (Game|GetPlayerCameraManager 0))
  ;[0.15 0.15 0.15 0.5] Set Camera Limit
  (Variables|/Script/Engine.PlayerCameraManager|SetViewPitchMin _returnvalue -55.0)
  (Variables|/Script/Engine.PlayerCameraManager|SetViewPitchMax _returnvalue 3e+01))

(event Collision|EventActorBeginOverlap
  (params (OtherActor :type Actor%20Object%20Reference)))

(event EventTick
  (params (DeltaSeconds :type Float%20%28single-precision%29))
  (bind _returnvalue (Pawn|GetControlRotation :!class /Script/Engine.Pawn))
  (bind _returnvalue_2 (Transformation|GetVelocity))
  (bind _charactermovement (Variables|Character|GetCharacterMovement))
  (bind _returnvalue_3 (Math|Vector|Normalize _returnvalue_2))
  (bind _returnvalue_4 (Math|Trig|DegreesToRadians (.yaw _returnvalue)))
  ;[0.15 0.15 0.15 0.5] Actor의 진행 방향과 Controller의 Roll vector dot product
  ;;[0.15 0.15 0.15 0.5] Controller 2D 진행 방향 벡터 (좌, 우)
  (bind _output_get (Variables|Default|SetControllerVector2D (Math|Vector2D|MakeVector2D (Math|Trig|Cos(Radians) _returnvalue_4) (Math|Trig|Sin(Radians) _returnvalue_4))))
  ;;[0.15 0.15 0.15 0.5] Actor 진행 방향 벡터 (좌, 우)
  (bind _output_get_2 (Variables|Default|SetActorVector2D (Math|Vector2D|MakeVector2D (.x _returnvalue_3) (.y _returnvalue_3))))
  (if (> (Math|Vector2D|DotProduct(2D) _output_get _output_get_2) (Variables|Default|GetStrafingDotConstant))
    (Variables|/Script/Engine.CharacterMovementComponent|SetbUseControllerDesiredRotation _charactermovement true :!label _label)
    (Variables|/Script/Engine.CharacterMovementComponent|SetbOrientRotationToMovement _charactermovement false)
    (elif (Variables|Default|GetbZooming)
      (goto _label)
      (else
        (Variables|/Script/Engine.CharacterMovementComponent|SetbUseControllerDesiredRotation _charactermovement false)
        (Variables|/Script/Engine.CharacterMovementComponent|SetbOrientRotationToMovement _charactermovement true)))))

(event EventControllerChanged
  (params (OldController :type Controller%20Object%20Reference) (NewController :type Controller%20Object%20Reference))
  ;[0.15 0.15 0.15 0.5] Add Enhanced Input to Mapping Context
  (bind _aspc_player_controller (Utilities|Casting|CastToPC_PlayerController NewController))
  (if (Utilities|IsValid (PlayerController|LocalPlayerSubsystems|GetEnhancedInputLocalPlayerSubsystem _aspc_player_controller))
    (Input|AddMappingContext (PlayerController|LocalPlayerSubsystems|GetEnhancedInputLocalPlayerSubsystem _aspc_player_controller) "/Game/Player/Input/IMC_Player.IMC_Player" 0 "(bIgnoreAllPressedKeysUntilRelease=True,bForceImmediately=False,bNotifyUserSettings=False)")
    (else
      (Development|PrintString "Couldn't Get Enhanced Input Local Player Subsystem"))))

(fn ConstructionScript)