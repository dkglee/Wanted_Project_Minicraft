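; BP_Arrow is an arrow projectile that flies in a gravity arc and damages iron golem monsters.
; Tick adds gravity to its velocity, moves it without sweep, faces it along that velocity, and destroys it once its lifetime runs out.
; Any overlap with its Box destroys the arrow and prints the other actor's name, but only a bp_ironGolem receives MonsterDamagedMessage with the arrow's damage.
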(event OnComponentBeginOverlap(Box)
  (params (OverlappedComponent :type Primitive%20Component%20Object%20Reference) (OtherActor :type Actor%20Object%20Reference) (OtherComp :type Primitive%20Component%20Object%20Reference) (OtherBodyIndex :type Integer) (bFromSweep :type Boolean) (SweepResult :type Hit%20Result%20Structure%20%28by%20ref%29))
  (Actor|DestroyActor)
  (Development|PrintString (Utilities|GetDisplayName OtherActor))
  (bind _asbp_iron_golem (Utilities|Casting|CastTobp_ironGolem OtherActor))
  (Class|BpiFight|MonsterDamaged(Message) _asbp_iron_golem (Variables|Default|GetDamage) "test_MAX"))

(event EventBeginPlay)

(event Collision|EventActorBeginOverlap
  (params (OtherActor :type Actor%20Object%20Reference)))

(event EventTick
  (params (DeltaSeconds :type Float%20%28single-precision%29))
  (bind _output_get (Variables|Default|SetCurrLifeTime (+ DeltaSeconds (Variables|Default|GetCurrLifeTime))))
  (if (> _output_get (Variables|Default|GetMaxLifeTime))
    (Variables|Default|SetCurrLifeTime 0.0)
    (Actor|DestroyActor)
    (else
      (Variables|Default|SetFixed%20Vector%20with%20Speed (+ (Variables|Default|GetFixed%20Vector%20with%20Speed) (* DeltaSeconds (Variables|Default|GetGravity))))
      (Transformation|SetActorLocation (+ (* DeltaSeconds (+ (Variables|Default|GetFixed%20Vector%20with%20Speed) (* DeltaSeconds (Variables|Default|GetGravity)))) (Transformation|GetActorLocation)) false false)
      (Transformation|SetActorRotation (Math|Conversions|RotationFromXVector (Variables|Default|GetFixed%20Vector%20with%20Speed))))))

(fn ConstructionScript)