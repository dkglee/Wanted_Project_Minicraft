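; Player basic skill that fires a three-arrow spread, powered by charge time up to a maximum.
; ActivateSkill projects a horizontal reach from direction, power and time limit, adding a scaled vertical component.
; GetVectorWithVelocity builds the two side vectors by tangent offset at plus and minus a set angle, rotated into world space.
; SpawnArrow spawns each BP_Arrow facing its vector, sets its velocity and travel, and links a new BP_BasicSkillEffect.
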(event EventBeginPlay)

(event Collision|EventActorBeginOverlap
  (params (OtherActor :type Actor%20Object%20Reference)))

(event EventTick
  (params (DeltaSeconds :type Float%20%28single-precision%29)))

(fn ConstructionScript
  (|CallParentFunction))

(fn ActivateSkill
  (params (ChargeTime :type Float%20%28double-precision%29) (Direction :type Vector :default "0, 0, 0") (Origin :type Vector :default "0, 0, 0") (SpawnTransform :type Transform))
  (bind _defaultspeed (Variables|Default|GetDefaultSpeed))
  (bind _max_power (Variables|Default|GetMax%20Power))
  (bind _angleasdegree (Variables|Default|GetAngleAsDegree))
  (bind _returnvalue (* ChargeTime _defaultspeed))
  (if (> _returnvalue _max_power)
    (Variables|Default|SetPower _max_power)
    (else
      (Variables|Default|SetPower _returnvalue)))
  (LocalVariables|SetOriginPoint Origin)
  (bind _ret (CallFunction|GetMaxDistance (Math|Vector2D|MakeVector2D (.x (LocalVariables|GetOriginPoint)) (.y (LocalVariables|GetOriginPoint))) (Math|Vector2D|MakeVector2D (.x Direction) (.y Direction)) (Variables|Default|GetPower)))
  (bind _output_get (Variables|Default|SetBasisVector (- _ret (Math|Vector2D|MakeVector2D (.x (LocalVariables|GetOriginPoint)) (.y (LocalVariables|GetOriginPoint))))))
  (Utilities|FlowControl|Sequence
    (:then_0
      (CallFunction|SpawnArrow (Math|Vector|MakeVector (.x _output_get) (.y _output_get) (* (Variables|Default|GetLimitTime) (* (.z Direction) (Variables|Default|GetPower)))) SpawnTransform))
    (:then_1
      (bind _retvector (CallFunction|GetVectorwithVelocity (* _angleasdegree -1.0) (Variables|Default|GetBasisVector) (LocalVariables|GetOriginPoint) (* (Variables|Default|GetLimitTime) (* (.z Direction) (Variables|Default|GetPower)))))
      (CallFunction|SpawnArrow _retvector SpawnTransform))
    (:then_2
      (bind _retvector_2 (CallFunction|GetVectorwithVelocity _angleasdegree (Variables|Default|GetBasisVector) (LocalVariables|GetOriginPoint) (* (Variables|Default|GetLimitTime) (* (.z Direction) (Variables|Default|GetPower)))))
      (CallFunction|SpawnArrow _retvector_2 SpawnTransform))))

(fn GetMaxDistance
  (params (Origin :type Vector%202D%20Structure) (Direction :type Vector%202D%20Structure) (Power :type Float%20%28double-precision%29))
  (return (+ Origin (* (* (Math|Vector2D|Normalize2D Direction) Power) (Variables|Default|GetLimitTime)))))

(fn GetVectorwithVelocity
  (params (AndgleAsDegree :type Float%20%28double-precision%29) (BasisVector :type Vector%202D%20Structure) (Origin :type Vector) (DirectionZ :type Float%20%28double-precision%29))
  (LocalVariables|SetLocalCoordinateVector (Math|Vector2D|MakeVector2D (Math|Float|Sqrt (+ (Math|Float|Square (.x BasisVector)) (Math|Float|Square (.y BasisVector)))) 0.0))
  (LocalVariables|SetRadianForWorld (Math|Trig|Atan2(Radians) (.y BasisVector) (.x BasisVector)))
  (bind _output_get (LocalVariables|SetTanzentedValue (* (.x (LocalVariables|GetLocalCoordinateVector)) (Math|Trig|Tan(Radians) (Math|Trig|DegreesToRadians AndgleAsDegree)))))
  (bind _output_get_2 (LocalVariables|SetLocalCoordinateVector (Math|Vector2D|MakeVector2D (.x (LocalVariables|GetLocalCoordinateVector)) _output_get)))
  ;[0.15 0.15 0.15 0.5] Destination in World Coordinate System
  (bind _output_get_3 (LocalVariables|SetPointInWorldCoordinate (+ (Math|Vector|MakeVector (.x (Class|KismetMathLibrary|GetRotated2D _output_get_2 (Math|Trig|RadiansToDegrees (LocalVariables|GetRadianForWorld)))) (.y (Class|KismetMathLibrary|GetRotated2D _output_get_2 (Math|Trig|RadiansToDegrees (LocalVariables|GetRadianForWorld)))) 0.0) Origin)))
  (Development|PrintString (Utilities|String|ToString(Vector) (+ (- _output_get_3 Origin) (Math|Vector|MakeVector 0.0 0.0 DirectionZ))))
  ;[0.15 0.15 0.15 0.5] Final Vector With Size
  (return (+ (- _output_get_3 Origin) (Math|Vector|MakeVector 0.0 0.0 DirectionZ))))

(fn SpawnArrow
  (params (FixedVector :type Vector) (SpawnTransform :type Transform))
  (bind _returnvalue (Math|Vector|Normalize FixedVector))
  (bind _returnvalue_2 (Math|Conversions|RotationFromXVector _returnvalue))
  (bind _returnvalue_3 (Game|SpawnActorfromClass "/Game/Player/BluePrints/Skill/BP_Arrow.BP_Arrow_C" (Math|Transform|MakeTransform (.location SpawnTransform) _returnvalue_2 (.scale SpawnTransform)) "Undefined" "MultiplyWithRoot" self 0))
  (if (Utilities|IsValid _returnvalue_3)
    (bind _output_get (Variables|/Game/Player/BluePrints/Skill/BP_Arrow.BP_Arrow_C|SetFixed%20Vector%20with%20Speed _returnvalue_3 FixedVector))
    (Variables|/Game/Player/BluePrints/Skill/BP_Arrow.BP_Arrow_C|SetMax%20Travel _returnvalue_3 _output_get)
    (Variables|/Game/Player/BluePrints/Skill/BP_Arrow.BP_Arrow_C|SetSpawnedTransform _returnvalue_3 (Math|Transform|MakeTransform (.location SpawnTransform) _returnvalue_2 (.scale SpawnTransform)))
    (bind _returnvalue_4 (Game|SpawnActorfromClass "/Game/Player/BluePrints/SkillEffects/BP_BasicSkillEffect.BP_BasicSkillEffect_C" (Math|Transform|MakeTransform "0, 0, 0" "0, 0, 0" "1.000000,1.000000,1.000000") "Undefined" "MultiplyWithRoot" self 0))
    (Variables|/Game/Player/BluePrints/Skill/BP_Arrow.BP_Arrow_C|SetSkillEffectPtr _returnvalue_3 _returnvalue_4)))