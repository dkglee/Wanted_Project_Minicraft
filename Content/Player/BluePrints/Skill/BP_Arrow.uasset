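; BP_Arrow is a player skill arrow projectile that damages iron golems.
; Tick moves it manually without sweep, adding gravity to its velocity, aligning rotation to travel direction and destroying it after a maximum lifetime.
; Box overlap with a bp_ironGolem triggers the skill effect, sends damage with a spawned BP_SkillBaseAttacked as hit pattern, then destroys the arrow.
; Overlapping any other actor stops it in place until its lifetime expires.
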(event OnComponentBeginOverlap(Box)
  (params (OverlappedComponent :type Primitive%20Component%20Object%20Reference) (OtherActor :type Actor%20Object%20Reference) (OtherComp :type Primitive%20Component%20Object%20Reference) (OtherBodyIndex :type Integer) (bFromSweep :type Boolean) (SweepResult :type Hit%20Result%20Structure%20%28by%20ref%29))
  (Development|PrintString (Utilities|String|ToString(Vector) (.impactpoint SweepResult)))
  (if (not (Variables|Default|GetbStopped))
    (bind _asbp_iron_golem (Utilities|Casting|CastTobp_ironGolem OtherActor)
      (:then
        (bind _asbp_askill_effect (Utilities|Casting|CastToBP_ASkillEffect (Variables|Default|GetSkillEffectPtr)))
        (Default|SpawnEffect _asbp_askill_effect (.location (Variables|Default|GetSpawnedTransform)) (Transformation|GetActorLocation))
        (bind _returnvalue (Game|SpawnActorfromClass "/Game/DamagedPattern/Blueprints/BP_SkillBaseAttacked.BP_SkillBaseAttacked_C" (Math|Transform|MakeTransform "0, 0, 0" "0, 0, 0" "1.000000,1.000000,1.000000") "Undefined" "MultiplyWithRoot" 0 0))
        (Class|BpiFight|MonsterDamaged(Message) _asbp_iron_golem (Variables|Default|GetDamage) "test_MAX" _returnvalue self)
        (Actor|DestroyActor))
      (:CastFailed
        (Variables|Default|SetbStopped true)))))

(event EventBeginPlay)

(event Collision|EventActorBeginOverlap
  (params (OtherActor :type Actor%20Object%20Reference)))

(event EventTick
  (params (DeltaSeconds :type Float%20%28single-precision%29))
  (bind _output_get (Variables|Default|SetCurrLifeTime (+ DeltaSeconds (Variables|Default|GetCurrLifeTime))))
  (if (> _output_get (Variables|Default|GetMaxLifeTime))
    (Variables|Default|SetCurrLifeTime 0.0)
    (Actor|DestroyActor)
    (elif (not (Variables|Default|GetbStopped))
      (Variables|Default|SetFixed%20Vector%20with%20Speed (+ (Variables|Default|GetFixed%20Vector%20with%20Speed) (* DeltaSeconds (Variables|Default|GetGravity))))
      (Transformation|SetActorLocation (+ (* DeltaSeconds (+ (Variables|Default|GetFixed%20Vector%20with%20Speed) (* DeltaSeconds (Variables|Default|GetGravity)))) (Transformation|GetActorLocation)) false false)
      (Transformation|SetActorRotation (Math|Conversions|RotationFromXVector (Variables|Default|GetFixed%20Vector%20with%20Speed))))))

(fn ConstructionScript)