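; BP_StrongSkill is a charged player skill that fires a fanned volley of BP_Arrow projectiles.
; ActivateSkill scales power by charge time up to a cap, then derives a center vector from direction and lifetime.
; It spawns one center arrow plus one per Angle entry, using tangent offsets rotated into world space.
; Each arrow receives its travel vector, effect actor, sound, random damage and a cycling volley index offset by 25.
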(event EventBeginPlay
  (|CallParentFunction) ; This node is disabled and will not be called.\nDrag off pins to build functionality.
)

(event Collision|EventActorBeginOverlap
  (params (OtherActor :type Actor%20Object%20Reference))
  (|CallParentFunction OtherActor) ; This node is disabled and will not be called.\nDrag off pins to build functionality.
)

(event EventTick
  (params (DeltaSeconds :type Float%20%28single-precision%29))
  (|CallParentFunction DeltaSeconds) ; This node is disabled and will not be called.\nDrag off pins to build functionality.
)

(fn ConstructionScript
  (|CallParentFunction))

(fn ActivateSkill
  (params (ChargeTime :type Float%20%28double-precision%29) (Direction :type Vector :default "0, 0, 0") (Origin :type Vector :default "0, 0, 0") (SpawnTransform :type Transform))
  (bind _max_power (Variables|Default|GetMax%20Power))
  (bind _defaultspeed (Variables|Default|GetDefaultSpeed))
  (bind _returnvalue (* ChargeTime _defaultspeed))
  (if (> _returnvalue _max_power)
    (Variables|Default|SetPower _max_power)
    (else
      (Variables|Default|SetPower _returnvalue)))
  (Variables|Default|SetOrigin%20Point Origin)
  (bind _ret (CallFunction|GetMaxDistance (Math|Vector2D|MakeVector2D (.x (Variables|Default|GetOrigin%20Point)) (.y (Variables|Default|GetOrigin%20Point))) (Math|Vector2D|MakeVector2D (.x Direction) (.y Direction)) (Variables|Default|GetPower)))
  (bind _output_get (Variables|Default|SetBasicVector (- _ret (Math|Vector2D|MakeVector2D (.x (Variables|Default|GetOrigin%20Point)) (.y (Variables|Default|GetOrigin%20Point))))))
  (Variables|Default|SetIndexOfArrow (Variables|Default|GetIndexOfArrow))
  (bind _result (Math|Integer|IncrementInt (Variables|Default|GetIndexOfArrow))
    (:%20%20
      (if (> _result 24)
        (Variables|Default|SetIndexOfArrow 0))
      (Utilities|FlowControl|Sequence
        (:then_0
          (CallFunction|SpawnArrow (Math|Vector|MakeVector (.x _output_get) (.y _output_get) (* (Variables|Default|GetLifeTime) (* (.z Direction) (Variables|Default|GetPower)))) SpawnTransform (+ (Variables|Default|GetIndexOfArrow) 25)))
        (:then_1
          (for _array_element (Variables|Default|GetAngle)
            (bind _retvector (CallFunction|GetVectorwithVelocity _array_element (Variables|Default|GetBasicVector) (Variables|Default|GetOrigin%20Point) (* (Variables|Default|GetLifeTime) (* (.z Direction) (Variables|Default|GetPower)))))
            (CallFunction|SpawnArrow _retvector SpawnTransform (+ (Variables|Default|GetIndexOfArrow) 25))))))))

(fn GetMaxDistance
  (params (Origin :type Vector%202D%20Structure) (Direction :type Vector%202D%20Structure) (Power :type Float%20%28double-precision%29))
  (return (+ Origin (* (* (Math|Vector2D|Normalize2D Direction) Power) (Variables|Default|GetLifeTime)))))

(fn GetVectorwithVelocity
  (params (AndgleAsDegree :type Float%20%28double-precision%29) (BasisVector :type Vector%202D%20Structure) (Origin :type Vector) (DirectionZ :type Float%20%28double-precision%29))
  (LocalVariables|SetLocalCoordinateVector (Math|Vector2D|MakeVector2D (Math|Float|Sqrt (+ (Math|Float|Square (.x BasisVector)) (Math|Float|Square (.y BasisVector)))) 0.0))
  (LocalVariables|SetRadianForWorld (Math|Trig|Atan2(Radians) (.y BasisVector) (.x BasisVector)))
  (bind _output_get (LocalVariables|SetTanzentedValue (* (.x (LocalVariables|GetLocalCoordinateVector)) (Math|Trig|Tan(Radians) (Math|Trig|DegreesToRadians AndgleAsDegree)))))
  (bind _output_get_2 (LocalVariables|SetLocalCoordinateVector (Math|Vector2D|MakeVector2D (.x (LocalVariables|GetLocalCoordinateVector)) _output_get)))
  (bind _output_get_3 (LocalVariables|SetPointInWorldCoordinate (+ (Math|Vector|MakeVector (.x (Class|KismetMathLibrary|GetRotated2D _output_get_2 (Math|Trig|RadiansToDegrees (LocalVariables|GetRadianForWorld)))) (.y (Class|KismetMathLibrary|GetRotated2D _output_get_2 (Math|Trig|RadiansToDegrees (LocalVariables|GetRadianForWorld)))) 0.0) Origin)))
  (return (+ (- _output_get_3 Origin) (Math|Vector|MakeVector 0.0 0.0 DirectionZ))))

(fn SpawnArrow
  (params (FixedVector :type Vector) (SpawnTransform :type Transform) (index :type Integer))
  (bind _returnvalue (Math|Vector|Normalize FixedVector))
  (bind _returnvalue_2 (Math|Conversions|RotationFromXVector _returnvalue))
  (bind _returnvalue_3 (Game|SpawnActorfromClass "/Game/Player/BluePrints/Skill/BP_Arrow.BP_Arrow_C" (Math|Transform|MakeTransform (.location SpawnTransform) _returnvalue_2 (.scale SpawnTransform)) "Undefined" "MultiplyWithRoot" self 0))
  (if (Utilities|IsValid _returnvalue_3)
    (bind _output_get (Variables|/Game/Player/BluePrints/Skill/BP_Arrow.BP_Arrow_C|SetFixed%20Vector%20with%20Speed _returnvalue_3 FixedVector))
    (Variables|/Game/Player/BluePrints/Skill/BP_Arrow.BP_Arrow_C|SetMax%20Travel _returnvalue_3 _output_get)
    (Variables|/Game/Player/BluePrints/Skill/BP_Arrow.BP_Arrow_C|SetSpawnedTransform _returnvalue_3 (Math|Transform|MakeTransform (.location SpawnTransform) _returnvalue_2 (.scale SpawnTransform)))
    (bind _returnvalue_4 (Game|SpawnActorfromClass "/Game/Player/BluePrints/SkillEffects/BP_BasicSkillEffect.BP_BasicSkillEffect_C" (Math|Transform|MakeTransform "0, 0, 0" "0, 0, 0" "1.000000,1.000000,1.000000") "Undefined" "MultiplyWithRoot" self 0))
    (Variables|/Game/Player/BluePrints/Skill/BP_Arrow.BP_Arrow_C|SetSkillEffectPtr _returnvalue_3 _returnvalue_4)
    (Variables|/Game/Player/BluePrints/Skill/BP_Arrow.BP_Arrow_C|SetSoundPtr _returnvalue_3 (Variables|Default|GetBP_SoundComponent))
    (Variables|/Game/Player/BluePrints/Skill/BP_Arrow.BP_Arrow_C|SetIndex _returnvalue_3 index)
    (Variables|/Game/Player/BluePrints/Skill/BP_Arrow.BP_Arrow_C|SetDamage _returnvalue_3 (Math|Random|RandomFloatinRange 1e+01 2e+01))))