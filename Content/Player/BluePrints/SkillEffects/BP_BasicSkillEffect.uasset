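; BP_BasicSkillEffect is a one-shot skill effect actor that plays a burst effect at a destination point.
; SpawnEffect, guarded by a DoOnce, moves the NSSimpleBurstLevel3 component to Dest, rotates it to face back toward Src, activates it and calls the parent implementation.
; It then triggers DestroyMySelf, which destroys the actor after a short delay.
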(event Custom|Destroy%20My%20Self
  (Utilities|FlowControl|Delay 2.0)
  (Actor|DestroyActor))

(event EventBeginPlay
  (|CallParentFunction) ; This node is disabled and will not be called.\nDrag off pins to build functionality.
)

(event Collision|EventActorBeginOverlap
  (params (OtherActor :type Actor%20Object%20Reference))
  (|CallParentFunction OtherActor) ; This node is disabled and will not be called.\nDrag off pins to build functionality.
)

(event EventTick
  (params (DeltaSeconds :type Float%20%28single-precision%29))
  (|CallParentFunction DeltaSeconds) ; This node is disabled and will not be called.\nDrag off pins to build functionality.
)

(fn ConstructionScript
  (|CallParentFunction))

(fn SpawnEffect
  (params (Src :type Vector :default "0, 0, 0") (Dest :type Vector :default "0, 0, 0"))
  (bind _ns_simple_burst_level_3 (Variables|Default|GetNS_Simple_Burst_Level_3))
  (Utilities|FlowControl|DoOnce false
    (:Completed
      (Transformation|SetWorldLocation _ns_simple_burst_level_3 Dest false false)
      (Transformation|SetWorldRotation _ns_simple_burst_level_3 (Math|Conversions|RotationFromXVector (Math|Vector|Normalize (- Src Dest))) false false)
      (Components|Activation|Activate _ns_simple_burst_level_3 true)
      (|CallParentFunction Src Dest)
      (CallFunction|DestroyMySelf))))