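; Player bow actor that fires skills on behalf of its parent BP_Steve character.
; On BeginPlay it binds to Steve's skill activation event.
; When the event fires, it fetches the requested skill from a BP_SkillFactory child actor and activates it with the charge time and attack direction.
; Skills spawn from the factory component's world transform, ignoring the passed controller origin; CreateSkillEvent is an empty stub.
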(event Custom|OnSkillActivated
  (params (ChargeTime :type Float%20%28double-precision%29) (E_Skill :type E_Skill%20Enum :default "NewEnumerator1") (AttackingDirection :type Vector) (ControllerOrigin :type Vector))
  (bind _asbp_skill_factory (Utilities|Casting|CastToBP_SkillFactory (Variables|/Script/Engine.ChildActorComponent|GetChildActor (Variables|Default|GetBP_SkillFactory))))
  (bind _retunskill (Default|GetSkill _asbp_skill_factory E_Skill))
  (Default|ActivateSkill _retunskill ChargeTime AttackingDirection (Transformation|GetWorldLocation (Variables|Default|GetBP_SkillFactory)) (Transformation|GetWorldTransform (Variables|Default|GetBP_SkillFactory))))

(event EventBeginPlay
  (bind _asbp_steve (Utilities|Casting|CastToBP_Steve (Actor|GetParentActor self)))
  (EventDispatchers|BindEventtoOnActivateSkill _asbp_steve (delegate Custom|OnSkillActivated)))

(event Collision|EventActorBeginOverlap
  (params (OtherActor :type Actor%20Object%20Reference)))

(event EventTick
  (params (DeltaSeconds :type Float%20%28single-precision%29)))

(fn ConstructionScript)

(fn CreateSkillEvent
  (params (Owner :type BP%20Steve%20Object%20Reference)))