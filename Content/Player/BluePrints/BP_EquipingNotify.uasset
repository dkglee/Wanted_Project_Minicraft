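; An animation notify that toggles the player's bow between equipped and unequipped at the point where it fires in an animation.
; It finds the bow through the BPBow child actor on the BP_Steve that owns the mesh.
; Based on the bow's Equipped flag, it detaches and reattaches it to the mesh's BowSocket or BowUnequipSocket, flips the flag and resets scale to one.
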(fn ReceivedNotify
  (params (MeshComp :type Skeletal%20Mesh%20Component%20Object%20Reference) (Animation :type Anim%20Sequence%20Base%20Object%20Reference) (EventReference :type Anim%20Notify%20Event%20Reference%20Structure%20%28by%20ref%29))
  (bind _asbp_steve (Utilities|Casting|CastToBP_Steve (Components|GetOwner MeshComp)))
  (bind _asbp_bow (Utilities|Casting|CastToBP_Bow (Variables|/Script/Engine.ChildActorComponent|GetChildActor (Variables|/Game/Player/BluePrints/BP_Steve.BP_Steve_C|GetBP_Bow _asbp_steve))))
  (if (not (Variables|/Game/Player/BluePrints/BP_Bow.BP_Bow_C|GetEquipped _asbp_bow))
    (Transformation|DetachFromActor _asbp_bow "KeepRelative" "KeepRelative" "KeepRelative")
    (Transformation|AttachComponentToComponent _asbp_bow MeshComp "BowSocket" "KeepRelative" "KeepRelative" "KeepRelative" true)
    (Variables|/Game/Player/BluePrints/BP_Bow.BP_Bow_C|SetEquipped _asbp_bow true)
    (else
      (Transformation|DetachFromActor _asbp_bow "KeepRelative" "KeepRelative" "KeepRelative")
      (Transformation|AttachComponentToComponent _asbp_bow MeshComp "BowUnequipSocket" "KeepRelative" "KeepRelative" "KeepRelative" true)
      (Variables|/Game/Player/BluePrints/BP_Bow.BP_Bow_C|SetEquipped _asbp_bow false)))
  (Transformation|SetActorScale3D _asbp_bow "1.000000,1.000000,1.000000")
  (return false))