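; Iron Golem monster character with its own viewport health bar and a telegraphed skill attack.
; The attack spawns a range indicator, waits out a charge, then plays a montage whose notify swaps the indicator for snow beam and throw skill actors.
; Capsule hits damage the player and launch them away by briefly switching to Flying and adding an impulse.
; Damage updates the bar; zero health disables movement, stops the montage and blocks new attacks.
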(event OnComponentHit(CapsuleComponent)
  (params (HitComponent :type Primitive%20Component%20Object%20Reference) (OtherActor :type Actor%20Object%20Reference) (OtherComp :type Primitive%20Component%20Object%20Reference) (NormalImpulse :type Vector :default "0, 0, 0") (Hit :type Hit%20Result%20Structure%20%28by%20ref%29))
  (bind _returnvalue (Actor|GetActorOfClass "/Game/Player/BluePrints/C_Player.C_Player_C"))
  (if (== OtherActor _returnvalue)
    (Utilities|IsValid _returnvalue
      (:Is%20Valid
        (Class|BpiFight|CharacterDamaged(Message) _returnvalue (Variables|Default|GethitDamage) "test_MAX")
        (Pawn|Components|CharacterMovement|SetMovementMode (Variables|/Script/Engine.Character|GetCharacterMovement _returnvalue) "MOVE_Flying" 0)
        (Physics|AddImpulse (Variables|/Script/Engine.Character|GetCharacterMovement _returnvalue) (* (Math|Vector|Normalize (- (Transformation|GetActorLocation _returnvalue) (- (Transformation|GetActorLocation) "0.000000,0.000000,200.000000"))) 3e+02) true)
        (Utilities|FlowControl|Delay 0.5)
        (Pawn|Components|CharacterMovement|SetMovementMode (Variables|/Script/Engine.Character|GetCharacterMovement _returnvalue) "MOVE_Walking" 0)))))

(event EventBeginPlay
  (bind _returnvalue (UserInterface|CreateWidget "/Game/monster/widget/wb_ironGolemHealth.wb_ironGolemHealth_C"))
  (UserInterface|Viewport|AddtoViewport _returnvalue 0)
  (bind _output_get (Variables|Default|SethealthUI _returnvalue))
  (Progress|SetPercent (Variables|/Game/monster/widget/wb_ironGolemHealth.wb_ironGolemHealth_C|GethealthBar _output_get) (/ (Variables|Default|Gethealth) 1e+02)))

(event EventTick
  (params (DeltaSeconds :type Float%20%28single-precision%29))
  (Variables|Default|SetmovingSpeed (Math|Vector|VectorLength (Transformation|GetVelocity))))

(event EventIronGolemAttack
  (if (not (Variables|Default|GetisDead))
    (if (not (Variables|Default|GetisAttacking))
      (bind _returnvalue (Game|SpawnActorfromClass "/Game/monster/skill/bp_skillRange.bp_skillRange_C" (Transformation|GetWorldTransform (Variables|Default|Getskill1Arrow1)) "Undefined" "MultiplyWithRoot" 0 0))
      (Variables|Default|SetskillRange _returnvalue)
      (Utilities|FlowControl|Delay (Variables|Default|Getskill1ChargingDuration))
      (Animation|Montage|PlayMontage (Variables|Character|GetMesh) "/Game/monster/animation/ironGolemMontage.ironGolemMontage" 0.8 0.0 "Default"
        (:then
          (Variables|Default|SetisAttacking true))
        (:OnCompleted
          (Variables|Default|SetisAttacking false))
        (:OnNotifyBegin
          (Utilities|IsValid (Variables|Default|GetskillRange)
            (:Is%20Valid
              (Actor|DestroyActor (Variables|Default|GetskillRange))
              (Game|SpawnActorfromClass "/Game/monster/skill/bp_skillSnowBeam.bp_skillSnowBeam_C" (Transformation|GetWorldTransform (Variables|Default|Getskill1EffectArrow)) "Undefined" "MultiplyWithRoot" 0 0)
              (Game|SpawnActorfromClass "/Game/monster/skill/bp_skillThrow.bp_skillThrow_C" (Transformation|GetWorldTransform (Variables|Default|Getskill1Arrow1)) "Undefined" "MultiplyWithRoot" 0 0))))))))

(event EventMonsterDamaged
  (params (damage :type Float%20%28double-precision%29) (type :type test%20Enum :default "test_MAX"))
  (bind _healthui (Variables|Default|GethealthUI))
  (bind _healthbar (Variables|/Game/monster/widget/wb_ironGolemHealth.wb_ironGolemHealth_C|GethealthBar _healthui))
  (Variables|Default|Sethealth (- (Variables|Default|Gethealth) damage))
  (if (<= (Variables|Default|Gethealth) 0.0)
    (Progress|SetPercent _healthbar 0.0)
    (Pawn|Components|CharacterMovement|DisableMovement (Variables|Character|GetCharacterMovement))
    (Variables|Default|SetisDead true)
    (Animation|StopAnimMontage "/Game/monster/animation/ironGolemMontage.ironGolemMontage")
    (else
      (Progress|SetPercent _healthbar (/ (Variables|Default|Gethealth) 1e+02)))))

(fn ConstructionScript)