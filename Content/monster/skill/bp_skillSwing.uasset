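; Swing skill actor for a monster, apparently the iron golem, that launches a moving damage box toward Steve.
; On BeginPlay it waits briefly, then a timeline slides it horizontally a fixed distance along the direction to Steve's position at that moment, before destroying itself.
; When the box overlaps Steve, it spawns a BP_swingPattern and passes it with the skill damage through CharacterDamagedMessage.
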(event OnComponentBeginOverlap(Box)
  (params (OverlappedComponent :type Primitive%20Component%20Object%20Reference) (OtherActor :type Actor%20Object%20Reference) (OtherComp :type Primitive%20Component%20Object%20Reference) (OtherBodyIndex :type Integer) (bFromSweep :type Boolean) (SweepResult :type Hit%20Result%20Structure%20%28by%20ref%29))
  (Utilities|Casting|CastToBP_Steve OtherActor)
  (bind _returnvalue (Game|SpawnActorfromClass "/Game/DamagedPattern/Blueprints/ironGolem/BP_swingPattern.BP_swingPattern_C" (Math|Transform|MakeTransform "0, 0, 0" "0, 0, 0" "1.000000,1.000000,1.000000") "Undefined" "MultiplyWithRoot" 0 0))
  (Class|BpiFight|CharacterDamaged(Message) OtherActor (Variables|Default|GetskillDamage) "test_MAX" _returnvalue))

(event EventBeginPlay
  (bind _returnvalue (Transformation|GetActorLocation))
  (bind _returnvalue_2 (Actor|GetActorOfClass "/Game/monster/bp_ironGolem.bp_ironGolem_C"))
  (Variables|Default|Setbp_ironGolem _returnvalue_2)
  (bind _returnvalue_3 (Actor|GetActorOfClass "/Game/Player/BluePrints/BP_Steve.BP_Steve_C"))
  (Variables|Default|Setbp_steve _returnvalue_3)
  (Utilities|FlowControl|Delay 1.0)
  (bind _output_get (Variables|Default|Setstart (Transformation|GetActorLocation)))
  (Variables|Default|Setend (+ (* (Math|Vector|Normalize (- (Math|Vector|MakeVector (.x (Transformation|GetActorLocation (Variables|Default|Getbp_steve))) (.y (Transformation|GetActorLocation (Variables|Default|Getbp_steve))) 0.0) (Math|Vector|MakeVector (.x _returnvalue) (.y _returnvalue) 0.0))) 2e+03) _output_get))
  (bind _newtrack_0 (Timeline|Timeline PlayFromStart)
    (:Update
      (Transformation|SetActorLocation (Math|Vector|MakeVector (Math|Float|Lerp (.x (Variables|Default|Getstart)) (.x (Variables|Default|Getend)) _newtrack_0) (Math|Float|Lerp (.y (Variables|Default|Getstart)) (.y (Variables|Default|Getend)) _newtrack_0) (.z (Variables|Default|Getstart))) false false))
    (:Finished
      (Utilities|FlowControl|Delay 0.5)
      (Actor|DestroyActor))))

(fn ConstructionScript)