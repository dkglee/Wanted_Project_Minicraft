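; Skill actor that makes the Iron Golem dash to where Steve stands when the actor spawns.
; On BeginPlay it finds both actors by class, saves their locations, and uses a Timeline to lerp the golem's X and Y, keeping its starting height.
; It destroys itself shortly after the dash finishes.
; The sphere overlap event is empty, and the damage and BP_dashPattern spawn logic is disconnected.
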(event OnComponentBeginOverlap(Sphere)
  (params (OverlappedComponent :type Primitive%20Component%20Object%20Reference) (OtherActor :type Actor%20Object%20Reference) (OtherComp :type Primitive%20Component%20Object%20Reference) (OtherBodyIndex :type Integer) (bFromSweep :type Boolean) (SweepResult :type Hit%20Result%20Structure%20%28by%20ref%29)))

(event EventBeginPlay
  (bind _returnvalue (Actor|GetActorOfClass "/Game/Player/BluePrints/BP_Steve.BP_Steve_C"))
  (Variables|Default|SetAs%20BP%20Steve _returnvalue)
  (bind _returnvalue_2 (Actor|GetActorOfClass "/Game/monster/bp_ironGolem.bp_ironGolem_C"))
  (Variables|Default|SetAs%20Bp%20Iron%20Golem _returnvalue_2)
  (Variables|Default|Setstart (Transformation|GetActorLocation (Variables|Default|GetAs%20Bp%20Iron%20Golem)))
  (Variables|Default|Setend (Transformation|GetActorLocation (Variables|Default|GetAs%20BP%20Steve)))
  (bind _time (Timeline|Timeline Play)
    (:Update
      (Transformation|SetActorLocation (Variables|Default|GetAs%20Bp%20Iron%20Golem) (Math|Vector|MakeVector (Math|Float|Lerp (.x (Variables|Default|Getstart)) (.x (Variables|Default|Getend)) _time) (Math|Float|Lerp (.y (Variables|Default|Getstart)) (.y (Variables|Default|Getend)) _time) (.z (Variables|Default|Getstart))) false false))
    (:Finished
      (Utilities|FlowControl|Delay 0.5)
      (Actor|DestroyActor))))

(event Collision|EventActorBeginOverlap
  (params (OtherActor :type Actor%20Object%20Reference)))

(event EventTick
  (params (DeltaSeconds :type Float%20%28single-precision%29)))

(fn ConstructionScript)