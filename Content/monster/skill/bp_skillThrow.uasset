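; Monster throw skill actor that damages what overlaps its Box and passes on a throw reaction.
; Each overlap spawns a BP_SkillThrowPattern, gives it the ThrowArrow, and sends it with SkillDamage through CharacterDamagedMessage to the overlapping actor.
; Tick turns off Cube collision shortly after spawn, while Box collision is left untouched.
; The actor destroys itself after SkillDuration.
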(event OnComponentBeginOverlap(Cube)
  (params (OverlappedComponent :type Primitive%20Component%20Object%20Reference) (OtherActor :type Actor%20Object%20Reference) (OtherComp :type Primitive%20Component%20Object%20Reference) (OtherBodyIndex :type Integer) (bFromSweep :type Boolean) (SweepResult :type Hit%20Result%20Structure%20%28by%20ref%29)))

(event OnComponentBeginOverlap(Box)
  (params (OverlappedComponent :type Primitive%20Component%20Object%20Reference) (OtherActor :type Actor%20Object%20Reference) (OtherComp :type Primitive%20Component%20Object%20Reference) (OtherBodyIndex :type Integer) (bFromSweep :type Boolean) (SweepResult :type Hit%20Result%20Structure%20%28by%20ref%29))
  (bind _returnvalue (Game|SpawnActorfromClass "/Game/DamagedPattern/Blueprints/ironGolem/BP_SkillThrowPattern.BP_SkillThrowPattern_C" (Math|Transform|MakeTransform "0, 0, 0" "0, 0, 0" "1.000000,1.000000,1.000000") "Undefined" "MultiplyWithRoot" 0 0))
  (Variables|/Game/DamagedPattern/Blueprints/ironGolem/BP_SkillThrowPattern.BP_SkillThrowPattern_C|SetThrowArrowTemp _returnvalue (Variables|Default|GetthrowArrow))
  (Class|BpiFight|CharacterDamaged(Message) OtherActor (Variables|Default|GetskillDamage) "test_MAX" _returnvalue))

(event EventBeginPlay
  (Utilities|FlowControl|Delay (Variables|Default|GetskillDuration))
  (Actor|DestroyActor))

(event EventTick
  (params (DeltaSeconds :type Float%20%28single-precision%29))
  (bind _output_get (Variables|Default|Settime (+ DeltaSeconds (Variables|Default|Gettime))))
  (if (> _output_get 0.2)
    (Collision|SetCollisionEnabled (Variables|Default|GetCube) "NoCollision")))

(fn ConstructionScript)