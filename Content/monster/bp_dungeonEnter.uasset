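; Dungeon entrance actor that teleports the player's BP_Steve character into and out of the dungeon, caching that character on BeginPlay.
; EnterDungeon fires the Enter event, which moves Steve to the Bp_dungeonSpawn arrow's location and rotation, then starts the BP_BossStartCamera sequence.
; ExitDungeon fires the Exit event, which returns Steve to this actor's own Arrow.
; Nothing here triggers on overlap; the Box check is unconnected debug printing.
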(event Custom|enter
  (bind _returnvalue (Actor|GetActorOfClass "/Game/monster/bp_dungeonSpawn.bp_dungeonSpawn_C"))
  (Transformation|SetActorLocationAndRotation (Variables|Default|GetAs%20BP%20Steve) (Transformation|GetWorldLocation (Variables|/Game/monster/bp_dungeonSpawn.bp_dungeonSpawn_C|GetArrow _returnvalue)) (Transformation|GetWorldRotation (Variables|/Game/monster/bp_dungeonSpawn.bp_dungeonSpawn_C|GetArrow _returnvalue)) false true)
  (bind _returnvalue_2 (Actor|GetActorOfClass "/Game/Player/Camera/BP_BossStartCamera.BP_BossStartCamera_C"))
  (Default|StartCamera _returnvalue_2))

(event Custom|exit
  (bind _arrow (Variables|Default|GetArrow))
  (Transformation|SetActorLocationAndRotation (Variables|Default|GetAs%20BP%20Steve) (Transformation|GetWorldLocation _arrow) (Transformation|GetWorldRotation _arrow) false true))

(event EventBeginPlay
  (bind _asbp_steve (Utilities|Casting|CastToBP_Steve (Game|GetPlayerCharacter 0)))
  (Variables|Default|SetAs%20BP%20Steve _asbp_steve))

(event Collision|EventActorBeginOverlap
  (params (OtherActor :type Actor%20Object%20Reference)))

(event EventTick
  (params (DeltaSeconds :type Float%20%28single-precision%29)))

(fn ConstructionScript)

(fn EnterDungeon
  (CallFunction|Enter))

(fn ExitDungeon
  (CallFunction|Exit))