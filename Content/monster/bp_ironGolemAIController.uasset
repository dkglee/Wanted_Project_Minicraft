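; AI controller for the iron golem monster that starts its behavior tree and detects the player.
; When pawn sensing spots Steve, it sets the blackboard flag for chase range.
; On the first sighting only, it adds the golem's health widget to the viewport, binds it to the controlled golem and refills the golem's health to max.
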(event OnSeePawn(PawnSensing)
  (params (Pawn :type Pawn%20Object%20Reference))
  (bind _asbp_steve (Utilities|Casting|CastToBP_Steve Pawn))
  (Variables|Default|SetAs%20BP%20Steve _asbp_steve)
  (AI|Components|Blackboard|SetValueasBool (AI|GetBlackboard 0) (Utilities|Name|MakeLiteralName "isPlayerinChaseRange") true)
  (Utilities|FlowControl|DoOnce false
    (:Completed
      (Variables|Default|SetisDetected true)
      (bind _returnvalue (UserInterface|CreateWidget "/Game/monster/widget/ingame/wb_ironGolem.wb_ironGolem_C"))
      (UserInterface|Viewport|AddtoViewport _returnvalue 0)
      (bind _output_get (Variables|Default|Setwb_ironGolem _returnvalue))
      (bind _asbp_iron_golem (Utilities|Casting|CastTobp_ironGolem (Pawn|GetControlledPawn)))
      (Variables|/Game/monster/widget/ingame/wb_ironGolemHealth.wb_ironGolemHealth_C|Setowner (Variables|/Game/monster/widget/ingame/wb_ironGolem.wb_ironGolem_C|Getwb_ironGolemHealth _output_get) _asbp_iron_golem)
      (Variables|/Game/monster/bp_ironGolem.bp_ironGolem_C|Sethealth _asbp_iron_golem (Variables|/Game/monster/bp_ironGolem.bp_ironGolem_C|GetmaxHealth _asbp_iron_golem)))))

(event EventBeginPlay
  (AI|RunBehaviorTree "/Game/monster/bt_ironGolem.bt_ironGolem"))

(event EventTick
  (params (DeltaSeconds :type Float%20%28single-precision%29)))

(fn ConstructionScript)