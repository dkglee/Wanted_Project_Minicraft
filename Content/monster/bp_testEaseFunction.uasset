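; Test actor in the monster folder that tries out an easing motion by moving Sphere toward Sphere1's height.
; EaseInBounceFunc triggers a timeline that lerps Z from Sphere's current height each update.
; X uses a circular-ease square-root formula on that lerped Z, not on normalized alpha, despite the bounce name.
; Each update spawns a particle at Sphere and prints a scaled-down X for debugging.
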(event Custom|easeInBounce
  (bind _newtrack_0 (Timeline|Timeline Play)
    (:Update
      (Transformation|SetRelativeLocation (Variables|Default|GetSphere) (Math|Vector|MakeVector (Math|Float|Sqrt (- 1.0 (Math|Float|Power (- 1.0 (Math|Float|Lerp (.z (Variables|/Script/Engine.SceneComponent|GetRelativeLocation (Variables|Default|GetSphere))) (.z (Variables|/Script/Engine.SceneComponent|GetRelativeLocation (Variables|Default|GetSphere1))) _newtrack_0)) 2.0))) 0.0 (Math|Float|Lerp (.z (Variables|/Script/Engine.SceneComponent|GetRelativeLocation (Variables|Default|GetSphere))) (.z (Variables|/Script/Engine.SceneComponent|GetRelativeLocation (Variables|Default|GetSphere1))) _newtrack_0)) false false)
      (Effects|SpawnEmitteratLocation "/Engine/Tutorial/SubEditors/TutorialAssets/TutorialParticleSystem.TutorialParticleSystem" (Transformation|GetWorldLocation (Variables|Default|GetSphere)))
      (Development|PrintString (Utilities|String|ToString(Float) (/ (Math|Float|Sqrt (- 1.0 (Math|Float|Power (- 1.0 (Math|Float|Lerp (.z (Variables|/Script/Engine.SceneComponent|GetRelativeLocation (Variables|Default|GetSphere))) (.z (Variables|/Script/Engine.SceneComponent|GetRelativeLocation (Variables|Default|GetSphere1))) _newtrack_0)) 2.0))) 1e+07))))))

(event EventBeginPlay
  (Variables|Default|SetNewVar (Transformation|GetWorldLocation (Variables|Default|GetSphere))))

(event Collision|EventActorBeginOverlap
  (params (OtherActor :type Actor%20Object%20Reference)))

(event EventTick
  (params (DeltaSeconds :type Float%20%28single-precision%29)))

(fn ConstructionScript)

(fn EaseinBounceFunc
  (CallFunction|EaseinBounce))