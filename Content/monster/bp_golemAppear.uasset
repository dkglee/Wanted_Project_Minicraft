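; Golem appearance intro actor that plays a short camera cutscene before gameplay begins.
; Its start event switches the player's view to itself, plays the skeletal mesh animation in slow motion, then pauses it and shows a timed start widget.
; It then removes the widget, flags BP_Steve's game as started, initializes his widget and returns the view to him.
; The camera-move event is an empty stub, and a Test function triggers the sequence.
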(event Custom|cameraMove)

(event Custom|start
  (bind _skeletalmesh (Variables|Default|GetSkeletalMesh))
  (Game|Player|SetViewTargetwithBlend (Game|GetPlayerController 0) self 0.0 "VTBlend_Linear" 0.0 false)
  (CallFunction|CameraMove)
  (Components|Timeline|SetPlayRate _skeletalmesh 0.2)
  (Audio|Components|Audio|Play _skeletalmesh false)
  (Utilities|FlowControl|Delay 1.75)
  (Variables|/Script/Engine.SkeletalMeshComponent|SetbPauseAnims _skeletalmesh true)
  (bind _returnvalue (UserInterface|CreateWidget "/Game/monster/widget/start_end/wb_start.wb_start_C"))
  (UserInterface|Viewport|AddtoViewport _returnvalue 0)
  (Utilities|FlowControl|Delay 5.0)
  (Widget|RemovefromParent _returnvalue)
  (bind _returnvalue_2 (Actor|GetActorOfClass "/Game/Player/BluePrints/BP_Steve.BP_Steve_C"))
  (Variables|/Game/Player/BluePrints/BP_Steve.BP_Steve_C|SetbGameStart _returnvalue_2 true)
  (Default|InitializeWidget _returnvalue_2)
  (Game|Player|SetViewTargetwithBlend (Game|GetPlayerController 0) _returnvalue_2 0.0 "VTBlend_Linear" 0.0 false))

(event EventBeginPlay)

(event Collision|EventActorBeginOverlap
  (params (OtherActor :type Actor%20Object%20Reference)))

(event EventTick
  (params (DeltaSeconds :type Float%20%28single-precision%29)))

(fn ConstructionScript)

(fn Test
  (CallFunction|Start))